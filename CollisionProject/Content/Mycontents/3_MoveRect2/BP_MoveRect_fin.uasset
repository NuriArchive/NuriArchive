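; Actor Blueprint that moves its Cone component around a square loop in the relative XZ plane while IsMove is true.
; Tick switches on the Movetype enum and passes Speed scaled by DeltaSeconds to one function per direction (right, up, left, down).
; Each function offsets the cone and advances Movetype when it crosses that side's limit, forming a simple state machine.
; An unconnected inline version and an earlier function set without state changes remain unused.
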(event `self.ReceiveTick`
  (params (DeltaSeconds :type "Float (single-precision)"))
  (bind _returnvalue (* DeltaSeconds (`self.speed`)))
  (bind _returnvalue_2 (* _returnvalue -1.0))
  (if (`self.IsMove`)
    (switch `/Game/Mycontents/EN_w` (`self.movetype`)
      (:`NewEnumerator0`
        (`self.우로 이동 1` _returnvalue))
      (:`NewEnumerator1`
        (`self.위로 이동 1` _returnvalue))
      (:`NewEnumerator2`
        (`self.좌로 이동 1` _returnvalue_2))
      (:`NewEnumerator3`
        (`self.아래로 이동 1` _returnvalue_2)))))

(fn `UserConstructionScript`)

(fn `아래로 이동`
  (params (DeltaLocation_Z :type "Float (double-precision)"))
  (bind _cone (`self.cone`))
  (bind (_relativelocation_x _relativelocation_y _relativelocation_z) (`KismetMathLibrary.BreakVector` (`SceneComponent.RelativeLocation` _cone)))
  (`SceneComponent.K2_AddRelativeLocation` _cone (`KismetMathLibrary.MakeVector` 0.0 0.0 DeltaLocation_Z) false false)
  (if (<= _relativelocation_z 0.0)
    _))

(fn `아래로 이동 1`
  (params (DeltaLocation_Z :type "Float (double-precision)"))
  (bind _cone (`self.cone`))
  (bind (_relativelocation_x _relativelocation_y _relativelocation_z) (`KismetMathLibrary.BreakVector` (`SceneComponent.RelativeLocation` _cone)))
  (`SceneComponent.K2_AddRelativeLocation` _cone (`KismetMathLibrary.MakeVector` 0.0 0.0 DeltaLocation_Z) false false)
  (if (<= _relativelocation_z 0.0)
    (set `self.movetype` "NewEnumerator0")))

(fn `우로 이동`
  (params (DeltaLocation_X :type "Float (double-precision)"))
  (bind _cone (`self.cone`))
  (bind _relativelocation_x (`KismetMathLibrary.BreakVector` (`SceneComponent.RelativeLocation` _cone)))
  (`SceneComponent.K2_AddRelativeLocation` _cone (`KismetMathLibrary.MakeVector` DeltaLocation_X) false false)
  (if (>= _relativelocation_x 500.0)
    _))

(fn `우로 이동 1`
  (params (DeltaLocation_X :type "Float (double-precision)"))
  (bind _cone (`self.cone`))
  (bind _relativelocation_x (`KismetMathLibrary.BreakVector` (`SceneComponent.RelativeLocation` _cone)))
  (`SceneComponent.K2_AddRelativeLocation` _cone (`KismetMathLibrary.MakeVector` DeltaLocation_X) false false)
  (if (>= _relativelocation_x 500.0)
    (set `self.movetype` "NewEnumerator1")))

(fn `위로 이동`
  (params (DeltaLocation_Z :type "Float (double-precision)"))
  (bind _cone (`self.cone`))
  (bind (_relativelocation_x _relativelocation_y _relativelocation_z) (`KismetMathLibrary.BreakVector` (`SceneComponent.RelativeLocation` _cone)))
  (`SceneComponent.K2_AddRelativeLocation` _cone (`KismetMathLibrary.MakeVector` 0.0 0.0 DeltaLocation_Z) false false)
  (if (>= _relativelocation_z 500.0)
    _))

(fn `위로 이동 1`
  (params (DeltaLocation_Z :type "Float (double-precision)"))
  (bind _cone (`self.cone`))
  (bind (_relativelocation_x _relativelocation_y _relativelocation_z) (`KismetMathLibrary.BreakVector` (`SceneComponent.RelativeLocation` _cone)))
  (`SceneComponent.K2_AddRelativeLocation` _cone (`KismetMathLibrary.MakeVector` 0.0 0.0 DeltaLocation_Z) false false)
  (if (>= _relativelocation_z 500.0)
    (set `self.movetype` "NewEnumerator2")))

(fn `좌로 이동`
  (params (DeltaLocation_X :type "Float (double-precision)"))
  (bind _cone (`self.cone`))
  (bind _relativelocation_x (`KismetMathLibrary.BreakVector` (`SceneComponent.RelativeLocation` _cone)))
  (`SceneComponent.K2_AddRelativeLocation` _cone (`KismetMathLibrary.MakeVector` DeltaLocation_X) false false)
  (if (<= _relativelocation_x 0.0)
    _))

(fn `좌로 이동 1`
  (params (DeltaLocation_X :type "Float (double-precision)"))
  (bind _cone (`self.cone`))
  (bind _relativelocation_x (`KismetMathLibrary.BreakVector` (`SceneComponent.RelativeLocation` _cone)))
  (`SceneComponent.K2_AddRelativeLocation` _cone (`KismetMathLibrary.MakeVector` DeltaLocation_X) false false)
  (if (<= _relativelocation_x 0.0)
    (set `self.movetype` "NewEnumerator3")))