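; BP_MyBox is a box actor that switches the IsPlay flag on every BP_HelloActor in the level.
; Its Cube sets the flag true on begin overlap and false on end overlap, finding the actors with GetAllActorsOfClass each time without filtering the overlapping actor.
; Cube hits only print a debug string.
; Unconnected nodes hold experiments with hiding, destroying, disabling collision and overlap logging.
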(event `self.Cube.OnComponentBeginOverlap`
  (params (OverlappedComponent :type "PrimitiveComponent Object Reference") (OtherActor :type "Actor Object Reference") (OtherComp :type "PrimitiveComponent Object Reference") (OtherBodyIndex :type Integer) (bFromSweep :type Boolean) (SweepResult :type "HitResult Structure (by ref)"))
  (bind _outactors (`GameplayStatics.GetAllActorsOfClass` "/Game/Mycontents/1_RightLeft/BP_HelloActor.BP_HelloActor_C"))
  (for _array_element _outactors
    (set `/Game/Mycontents/1_RightLeft/BP_HelloActor.IsPlay` true _array_element)))

(event `self.Cube.OnComponentEndOverlap`
  (params (OverlappedComponent :type "PrimitiveComponent Object Reference") (OtherActor :type "Actor Object Reference") (OtherComp :type "PrimitiveComponent Object Reference") (OtherBodyIndex :type Integer))
  (bind _outactors (`GameplayStatics.GetAllActorsOfClass` "/Game/Mycontents/1_RightLeft/BP_HelloActor.BP_HelloActor_C"))
  (for _array_element _outactors
    (set `/Game/Mycontents/1_RightLeft/BP_HelloActor.IsPlay` false _array_element)))

(event `self.Cube.OnComponentHit`
  (params (HitComponent :type "PrimitiveComponent Object Reference") (OtherActor :type "Actor Object Reference") (OtherComp :type "PrimitiveComponent Object Reference") (NormalImpulse :type "Vector Structure") (Hit :type "HitResult Structure (by ref)"))
  (`KismetSystemLibrary.PrintString` "Hello" true true (struct :`G` 0.66 :`B` 1.0 :`A` 1.0) 60.0))

(fn `UserConstructionScript`)