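; BP_MoveRect is an actor whose Cube component loops around a square path in the X-Z plane while IsPlay is set.
; Tick switches on the MoveType state, calling a direction function that offsets the cube by Speed times delta time and advances the state at each relative-location limit.
; Cube overlap and hit events print debug messages, and begin overlap also unhides the actor.
; Disconnected nodes hold alternative hide, destroy and collision-disable responses.
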(event `self.Cube.OnComponentBeginOverlap`
  (params (OverlappedComponent :type "PrimitiveComponent Object Reference") (OtherActor :type "Actor Object Reference") (OtherComp :type "PrimitiveComponent Object Reference") (OtherBodyIndex :type Integer) (bFromSweep :type Boolean) (SweepResult :type "HitResult Structure (by ref)"))
  (`KismetSystemLibrary.PrintString` (`KismetStringLibrary.Concat_StrStr` "BeginOverlap" "Overlapped Component" (`KismetSystemLibrary.GetDisplayName` OverlappedComponent) ", Other Actor :" (`KismetSystemLibrary.GetDisplayName` OtherActor) ", Other Comp :" (`KismetSystemLibrary.GetDisplayName` OtherComp)) true true (struct :`G` 0.66 :`B` 1.0 :`A` 1.0) 60.0)
  (`self.SetActorHiddenInGame` false))

(event `self.Cube.OnComponentEndOverlap`
  (params (OverlappedComponent :type "PrimitiveComponent Object Reference") (OtherActor :type "Actor Object Reference") (OtherComp :type "PrimitiveComponent Object Reference") (OtherBodyIndex :type Integer))
  (`KismetSystemLibrary.PrintString` (`KismetStringLibrary.Concat_StrStr` "EndOverlap" "Overlapped Component" (`KismetSystemLibrary.GetDisplayName` OverlappedComponent) ", Other Actor :" (`KismetSystemLibrary.GetDisplayName` OtherActor) ", Other Comp :" (`KismetSystemLibrary.GetDisplayName` OtherComp)) true true (struct :`R` 1.0 :`B` 0.030146 :`A` 1.0) 60.0))

(event `self.ReceiveTick`
  (params (DeltaSeconds :type "Float (single-precision)"))
  (bind _returnvalue (* DeltaSeconds (`self.Speed`)))
  (if (`self.isPlay`)
    (bind _output_get (set `self.MoveType` (`self.MoveType`)))
    (switch `/Game/Mycontents/EN_MoveType` _output_get
      (:`NewEnumerator0`
        (`self.MoveRight` _returnvalue))
      (:`NewEnumerator1`
        (`self.MoveUp` _returnvalue))
      (:`NewEnumerator2`
        (`self.MoveLeft` _returnvalue))
      (:`NewEnumerator3`
        (`self.MoveDown` _returnvalue)))))

(event `self.Cube.OnComponentHit`
  (params (HitComponent :type "PrimitiveComponent Object Reference") (OtherActor :type "Actor Object Reference") (OtherComp :type "PrimitiveComponent Object Reference") (NormalImpulse :type "Vector Structure") (Hit :type "HitResult Structure (by ref)"))
  (`KismetSystemLibrary.PrintString` (`KismetSystemLibrary.GetDisplayName` HitComponent)))

(fn `MoveDown`
  (params (A :type "Float (double-precision)"))
  (bind _cube (`self.Cube`))
  (bind (_relativelocation_x _relativelocation_y _relativelocation_z) (`KismetMathLibrary.BreakVector` (`SceneComponent.RelativeLocation` _cube)))
  ;[1 1 1] 아래로 이동
  (`SceneComponent.K2_AddRelativeLocation` _cube (`KismetMathLibrary.MakeVector` 0.0 0.0 (* A -1.0)) false false)
  (if (<= _relativelocation_z 0.0)
    (set `self.MoveType` "NewEnumerator0")))

(fn `MoveLeft`
  (params (A :type "Float (double-precision)"))
  (bind _cube (`self.Cube`))
  (bind _relativelocation_x (`KismetMathLibrary.BreakVector` (`SceneComponent.RelativeLocation` _cube)))
  ;[1 1 1] 좌로 이동
  (`SceneComponent.K2_AddRelativeLocation` _cube (`KismetMathLibrary.MakeVector` (* A -1.0)) false false)
  (if (<= _relativelocation_x 0.0)
    (set `self.MoveType` "NewEnumerator3")))

(fn `MoveRight`
  (params (DeltaLocation_X :type "Float (double-precision)"))
  (bind _cube (`self.Cube`))
  (bind _relativelocation_x (`KismetMathLibrary.BreakVector` (`SceneComponent.RelativeLocation` _cube)))
  ;[1 1 1] 우로 이동
  (`SceneComponent.K2_AddRelativeLocation` _cube (`KismetMathLibrary.MakeVector` DeltaLocation_X) false false)
  (if (>= _relativelocation_x 500.0)
    (set `self.MoveType` "NewEnumerator1")))

(fn `MoveUp`
  (params (DeltaLocation_Z :type "Float (double-precision)"))
  (bind _cube (`self.Cube`))
  (bind (_relativelocation_x _relativelocation_y _relativelocation_z) (`KismetMathLibrary.BreakVector` (`SceneComponent.RelativeLocation` _cube)))
  ;[1 1 1] 위로 이동
  (`SceneComponent.K2_AddRelativeLocation` _cube (`KismetMathLibrary.MakeVector` 0.0 0.0 DeltaLocation_Z) false false)
  (if (>= _relativelocation_z 500.0)
    (set `self.MoveType` "NewEnumerator2")))

(fn `UserConstructionScript`)