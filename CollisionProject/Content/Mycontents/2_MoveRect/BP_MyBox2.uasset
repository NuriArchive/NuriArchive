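; BP_MyBox2 is a trigger box actor that starts and stops every BP_MoveRect in the level.
; When its StaticMesh begins or ends an overlap, it gets all BP_MoveRect actors and sets their IsPlay to true or false, without filtering the overlapping actor.
; Hits on the mesh only print the hit component's name.
; Unconnected leftover nodes hold experiments with hiding, destroying, disabling collision and overlap debug printing.
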(event `self.StaticMesh.OnComponentBeginOverlap`
  (params (OverlappedComponent :type "PrimitiveComponent Object Reference") (OtherActor :type "Actor Object Reference") (OtherComp :type "PrimitiveComponent Object Reference") (OtherBodyIndex :type Integer) (bFromSweep :type Boolean) (SweepResult :type "HitResult Structure (by ref)"))
  (bind _outactors (`GameplayStatics.GetAllActorsOfClass` "/Game/Mycontents/2_MoveRect/BP_MoveRect.BP_MoveRect_C"))
  (for _array_element _outactors
    (set `/Game/Mycontents/2_MoveRect/BP_MoveRect.isPlay` true _array_element)))

(event `self.StaticMesh.OnComponentEndOverlap`
  (params (OverlappedComponent :type "PrimitiveComponent Object Reference") (OtherActor :type "Actor Object Reference") (OtherComp :type "PrimitiveComponent Object Reference") (OtherBodyIndex :type Integer))
  (bind _outactors (`GameplayStatics.GetAllActorsOfClass` "/Game/Mycontents/2_MoveRect/BP_MoveRect.BP_MoveRect_C"))
  (for _array_element _outactors
    (set `/Game/Mycontents/2_MoveRect/BP_MoveRect.isPlay` false _array_element)))

(event `self.StaticMesh.OnComponentHit`
  (params (HitComponent :type "PrimitiveComponent Object Reference") (OtherActor :type "Actor Object Reference") (OtherComp :type "PrimitiveComponent Object Reference") (NormalImpulse :type "Vector Structure") (Hit :type "HitResult Structure (by ref)"))
  (`KismetSystemLibrary.PrintString` (`KismetSystemLibrary.GetDisplayName` HitComponent)))

(fn `UserConstructionScript`)