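; BP_LeftRight is an actor that moves its Sphere component back and forth along its local X axis while playing.
; Tick moves the sphere at a constant, delta-time-scaled speed and flips the IsMove direction flag when it passes either limit around the origin.
; EventPlay and EventStop set the IsPlay flag that starts and pauses the motion.
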(event `self.ReceiveTick`
  (params (DeltaSeconds :type "Float (single-precision)"))
  (bind _returnvalue (* DeltaSeconds 100.0))
  (bind _sphere (`self.Sphere`))
  (bind _sphere_2 (`self.Sphere`))
  (bind _relativelocation_x (`KismetMathLibrary.BreakVector` (`SceneComponent.RelativeLocation` _sphere)))
  (bind _relativelocation_x_2 (`KismetMathLibrary.BreakVector` (`SceneComponent.RelativeLocation` _sphere_2)))
  (if (`self.IsPlay`)
    (if (`self.IsMove`)
      (`SceneComponent.K2_AddRelativeLocation` _sphere (`KismetMathLibrary.MakeVector` _returnvalue) false false)
      (if (>= _relativelocation_x 50.0)
        (set `self.IsMove` false))
      (else
        (`SceneComponent.K2_AddRelativeLocation` _sphere_2 (`KismetMathLibrary.MakeVector` (* _returnvalue -1.0)) false false)
        (if (<= _relativelocation_x_2 -50.0)
          (set `self.IsMove` true))))))

(event `/Game/MyContents/BPI_MoveActor.Event Play`
  (set `self.IsPlay` true))

(event `/Game/MyContents/BPI_MoveActor.Event Stop`
  (set `self.IsPlay` false))

(fn `UserConstructionScript`)