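; BP_Rect is an actor that moves its Pyramid component around a square loop in the local XZ plane.
; On Tick, an enum state switch (Right, Up, Left, Down) shifts the component at a constant speed and advances to the next side when a positional limit is reached.
; EventPlay and EventStop toggle the IsMove flag that starts and pauses the motion.
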(event `self.ReceiveTick`
  (params (DeltaSeconds :type "Float (single-precision)"))
  (bind _returnvalue (* DeltaSeconds 100.0))
  (bind _pyramid (`self.pyramid`))
  (bind _pyramid_2 (`self.pyramid`))
  (bind _pyramid_3 (`self.pyramid`))
  (bind _pyramid_4 (`self.pyramid`))
  (bind _returnvalue_2 (* _returnvalue -1.0))
  (bind _relativelocation_x (`KismetMathLibrary.BreakVector` (`SceneComponent.RelativeLocation` _pyramid_4)))
  (bind (_relativelocation_x_2 _relativelocation_y _relativelocation_z) (`KismetMathLibrary.BreakVector` (`SceneComponent.RelativeLocation` _pyramid)))
  (bind _relativelocation_x_3 (`KismetMathLibrary.BreakVector` (`SceneComponent.RelativeLocation` _pyramid_2)))
  (bind (_relativelocation_x_4 _relativelocation_y_2 _relativelocation_z_2) (`KismetMathLibrary.BreakVector` (`SceneComponent.RelativeLocation` _pyramid_3)))
  (if (`self.IsMove`)
    (switch `/Game/MyContents/EN_MoveType` (`self.Movetype`)
      (:`NewEnumerator0`
        (`SceneComponent.K2_AddRelativeLocation` _pyramid_2 (`KismetMathLibrary.MakeVector` _returnvalue) false false)
        (if (>= _relativelocation_x_3 100.0)
          (set `self.Movetype` "NewEnumerator1")))
      (:`NewEnumerator1`
        (`SceneComponent.K2_AddRelativeLocation` _pyramid_3 (`KismetMathLibrary.MakeVector` 0.0 0.0 _returnvalue) false false)
        (if (>= _relativelocation_z_2 100.0)
          (set `self.Movetype` "NewEnumerator2")))
      (:`NewEnumerator2`
        (`SceneComponent.K2_AddRelativeLocation` _pyramid_4 (`KismetMathLibrary.MakeVector` _returnvalue_2) false false)
        (if (<= _relativelocation_x -100.0)
          (set `self.Movetype` "NewEnumerator3")))
      (:`NewEnumerator3`
        (`SceneComponent.K2_AddRelativeLocation` _pyramid (`KismetMathLibrary.MakeVector` 0.0 0.0 _returnvalue_2) false false)
        (if (<= _relativelocation_z -100.0)
          (set `self.Movetype` "NewEnumerator0"))))))

(event `/Game/MyContents/BPI_MoveActor.Event Play`
  (set `self.IsMove` true))

(event `/Game/MyContents/BPI_MoveActor.Event Stop`
  (set `self.IsMove` false))

(fn `UserConstructionScript`)